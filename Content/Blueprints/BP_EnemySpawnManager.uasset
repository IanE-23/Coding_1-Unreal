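; BP_EnemySpawnManager runs enemy waves, starting a new one and dropping a key once the level is clear of enemies.
; NewEnemyWaveCheck, called with a transform, counts BP_Enemy actors and, if none remain, calls SpawnNewEnemies and spawns a BP_Key at that transform.
; SpawnNewEnemies waits briefly, then triggers every BP_EnemySpawner in the level.
; BeginPlay only reports the spawner count, and each step prints debug messages.
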(event Custom|NewEnemyWaveCheck
  (params (Transform :type Transform))
  (Development|PrintString "checking enemy count")
  (bind _outactors (Actor|GetAllActorsOfClass "/Game/Blueprints/BP_Enemy.BP_Enemy_C"))
  (if (> (Utilities|Array|Length _outactors) 0) ; if all enemies in the level are > 0, do nothing
    (Development|PrintString "There are still more enemies in the level")
    (else
      (Development|PrintString "Spawning enemies and a key")
      (CallFunction|SpawnNewEnemies)
      (Game|SpawnActorfromClass "/Game/Blueprints/BP_Key.BP_Key_C" Transform "Undefined" "MultiplyWithRoot" 0 0))))

(event Custom|SpawnNewEnemies
  (Development|PrintString "Spawning New Enemies in 4 seconds" true true "(R=0.277778,G=0.000000,B=0.004808,A=1.000000)")
  (Utilities|FlowControl|Delay 4.0)
  (bind _outactors (Actor|GetAllActorsOfClass "/Game/Blueprints/BP_EnemySpawner.BP_EnemySpawner_C"))
  (for (_array_element _array_index) _outactors
    (Default|SpawnNewEnemy _array_element)
    (Development|PrintString (Utilities|String|Append (Utilities|String|ToString(Integer) _array_index) ". " (Utilities|GetDisplayName _array_element) "is spawning...") true true "(R=0.621528,G=0.000000,B=0.018493,A=1.000000)" 5.0))
  (Development|PrintString "New Wave Complete!"))

(event EventBeginPlay
  (Development|PrintString "Spawn Manager is Active.")
  (bind _outactors (Actor|GetAllActorsOfClass "/Game/Blueprints/BP_EnemySpawner.BP_EnemySpawner_C")) ; Find all the spawner in the level
  (Development|PrintString (Utilities|String|Append " There are " (Utilities|String|ToString(Integer) (Utilities|Array|Length _outactors)) " spawners in the level." "There are" "##" "enemies in the level.") true true "(R=1.000000,G=0.000000,B=0.017000,A=1.000000)" 1e+01))

(fn ConstructionScript)