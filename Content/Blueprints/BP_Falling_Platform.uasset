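; BP_Falling_Platform is a platform that drops after the third-person character steps on it, then returns to its start.
; An overlap on the trigger box, while ready, plays an explosion sound and starts a delayed fall with physics simulation enabled.
; After a fall delay, physics turns off and a timeline lerps the platform back to its BeginPlay transform before re-arming it.
; Material swaps and debug prints mark each state.
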(event OnComponentBeginOverlap(BoxTrigger)
  (params (OverlappedComponent :type Primitive%20Component%20Object%20Reference) (OtherActor :type Actor%20Object%20Reference) (OtherComp :type Primitive%20Component%20Object%20Reference) (OtherBodyIndex :type Integer) (bFromSweep :type Boolean) (SweepResult :type Hit%20Result%20Structure%20%28by%20ref%29))
  (Development|PrintString "Something is on me. Get off")
  (Utilities|Casting|CastToBP_ThirdPersonCharacter OtherActor)
  (if (Variables|Default|GetIs%20Ready)
    (CallFunction|Activate)
    (else
      (Development|PrintString "The platform is not ready yet"))))

(event Custom|Activate
  (Audio|PlaySoundatLocation "/Game/StarterContent/Audio/Explosion01.Explosion01" (Transformation|GetWorldLocation (Variables|Default|GetPlatform)) "0, 0, 0" 1.0 1.0 0.0 0 0 0 0)
  (Variables|Default|SetIs%20Ready false)
  (Development|PrintString "Starting Countdown")
  (Rendering|Material|SetMaterial (Variables|Default|GetPlatform) 0 "/Game/Materials/Falling_Platform/MI_Active.MI_Active")
  (Utilities|FlowControl|Delay (Variables|PlatformSettings|GetFall%20Delay%20Duration)) ; wait half a second
  (CallFunction|Fall))

(event Custom|Fall
  (Development|PrintString "Falling")
  (Rendering|Material|SetMaterial (Variables|Default|GetPlatform) 0 "/Game/Materials/Falling_Platform/MI_Falling.MI_Falling")
  (Physics|SetSimulatePhysics (Variables|Default|GetPlatform) true) ; Allows platform to be affected by physics
  (Utilities|FlowControl|Delay (Variables|PlatformSettings|GetFall%20Duration))
  (CallFunction|Reset))

(event Custom|Reset
  (Development|PrintString "Platform is resetting")
  (Rendering|Material|SetMaterial (Variables|Default|GetPlatform) 0 "/Game/Materials/Falling_Platform/MI_Resetting.MI_Resetting")
  (Physics|SetSimulatePhysics (Variables|Default|GetPlatform) false) ; Allows platform to be affected by physics
  (Variables|Default|SetFallen%20Position (Transformation|GetWorldTransform (Variables|Default|GetPlatform)))
  (bind _newtrack_0 (Timeline|GoBackToStart PlayFromStart)
    (:Update
      (Transformation|SetWorldTransform (Variables|Default|GetPlatform) (Math|Transform|Lerp(Transform) (Variables|Default|GetFallen%20Position) (Variables|Default|GetStarting%20Transform) _newtrack_0) false false))
    (:Finished
      (Variables|Default|SetIs%20Ready true)
      (Development|PrintString "Platform is ready now")
      (Rendering|Material|SetMaterial (Variables|Default|GetPlatform) 0 "/Game/Materials/Falling_Platform/MI_Ready.MI_Ready"))))

(event EventBeginPlay
  (Variables|Default|SetStarting%20Transform (Transformation|GetWorldTransform (Variables|Default|GetPlatform))) ; capture the starting placement and rotation
)

(fn ConstructionScript)